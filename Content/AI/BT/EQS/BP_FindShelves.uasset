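; EQS context that picks a random BP_Shelves actor matching the querier's Category blackboard value.
; It scans all shelves in the level, adds matches to the ActorRef array without clearing it first, then writes a random entry to the PlaceRef blackboard key.
; The returned actor comes from a separate random index expression, so it can differ from the stored PlaceRef.
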(fn ProvideSingleActor
  (params (QuerierObject :type Object%20Object%20Reference) (QuerierActor :type Actor%20Object%20Reference))
  (bind _actorref (LocalVariables|GetActorRef))
  (bind _returnvalue (Utilities|Array|Length _actorref))
  (bind _returnvalue_2 (Math|Random|RandomInteger _returnvalue))
  (bind _output (Utilities|Array|Get(acopy) _actorref _returnvalue_2))
  (bind _outactors (Actor|GetAllActorsOfClass "/Game/AI/Blueprints/BP_Shelves.BP_Shelves_C"))
  (bind _array_element (Utilities|Array|ForEachLoopwithBreak _outactors)
    (:LoopBody
      (if (== (Math|Byte|MakeLiteralByte (Variables|/Game/AI/Blueprints/BP_Shelves.BP_Shelves_C|GetCategory _array_element)) (Class|BlackboardComponent|GetValueasEnum (AI|GetBlackboard QuerierActor) (Utilities|Name|MakeLiteralName "Category")))
        (Utilities|Array|AddUnique (LocalVariables|GetActorRef) _array_element)))
    (:Completed
      (AI|Components|Blackboard|SetValueasObject (AI|GetBlackboard QuerierActor) (Utilities|Name|MakeLiteralName "PlaceRef") _output)
      (return _output))))