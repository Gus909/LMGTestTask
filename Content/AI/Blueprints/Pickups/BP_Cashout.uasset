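; BP_Cashout is a cashout point that manages a queue of NPCs standing at positions defined by the child components of Queue.
; StartQueueTimer schedules MoveInQueue after a short delay unless that timer is already running.
; MoveInQueue removes the front NPC, then moves the rest forward by writing State and Point to their blackboards.
; It also clears component tags on queue points from the last assigned index onward.
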(event EventBeginPlay
  (Variables|Default|SetPointsRef (Components|GetChildrenComponents (Variables|Default|GetQueue) false)))

(event Collision|EventActorBeginOverlap
  (params (OtherActor :type Actor%20Object%20Reference)))

(event EventTick
  (params (DeltaSeconds :type Float%20%28single-precision%29)))

(fn ConstructionScript)

(fn MoveinQueue
  (bind _npcref (Variables|Default|GetNPCRef))
  (Utilities|Array|RemoveIndex _npcref)
  (for (_array_element _array_index) _npcref
    (LocalVariables|SetIndex _array_index)
    (AI|Components|Blackboard|SetValueasEnum (AI|GetBlackboard _array_element) (Utilities|Name|MakeLiteralName "State") (Utilities|Enum|LiteralenumE_AIState "NewEnumerator4"))
    (AI|Components|Blackboard|SetValueasVector (AI|GetBlackboard _array_element) (Utilities|Name|MakeLiteralName "Point") (Transformation|GetWorldLocation (Utilities|Array|Get(acopy) (Variables|Default|GetPointsRef) _array_index))))
  (for _index (range (LocalVariables|GetIndex) (- (Utilities|Array|Length (Variables|Default|GetPointsRef)) 1))
    (Utilities|Array|Clear (Variables|/Script/Engine.ActorComponent|GetComponentTags (Utilities|Array|Get(acopy) (Variables|Default|GetPointsRef) _index)))))

(fn StartQueueTimer
  (if (not (Utilities|Time|IsTimerActivebyHandle (Variables|Default|GetQueueTimer)))
    (bind _returnvalue (Utilities|Time|SetTimerbyFunctionName 0 "MoveInQueue" 4.0))
    (Variables|Default|SetQueueTimer _returnvalue)))