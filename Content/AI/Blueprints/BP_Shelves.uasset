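; BP_Shelves is a shelf actor that stocks itself with items of a randomly chosen category.
; On BeginPlay it picks the category, collects matching entries from the ClassOfItems class-to-category map, and spawns a random matching item at each of two spawn points.
; TakeItem finds the last valid spawned item, destroys it, removes it from the list and returns its class, using an index of 100 as the empty sentinel.
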(event EventBeginPlay
  (Variables|Default|SetCategory (Utilities|Enum|ByteToEnumE_Category (Math|Conversions|ToByte(Integer) (Math|Random|RandomInteger 3))))
  (CallFunction|FindClasses)
  (CallFunction|SpawnItems (Variables|Default|GetSpawnPoint))
  (CallFunction|SpawnItems (Variables|Default|GetSpawnPoint1)))

(event Collision|EventActorBeginOverlap
  (params (OtherActor :type Actor%20Object%20Reference)))

(event EventTick
  (params (DeltaSeconds :type Float%20%28single-precision%29)))

(fn ConstructionScript)

(fn FindClasses
  (bind _values (Utilities|Map|Values (Variables|Default|GetClassOfItems)))
  (for (_array_element _array_index) _values
    (if (== (Math|Byte|MakeLiteralByte _array_element) (Math|Byte|MakeLiteralByte (Variables|Default|GetCategory)))
      (Utilities|Array|AddUnique (Variables|Default|GetIndex%20Arr) _array_index))))

(fn SpawnItems
  (params (PlaceRef :type Scene%20Component%20Object%20Reference))
  (bind _keys (Utilities|Map|Keys (Variables|Default|GetClassOfItems)))
  (bind _returnvalue (Game|SpawnActorfromClass (Utilities|Array|Get(acopy) _keys (.OutItem (Utilities|Array|Random (Variables|Default|GetIndex%20Arr)))) (Transformation|GetWorldTransform PlaceRef) "AdjustIfPossibleButAlwaysSpawn" "MultiplyWithRoot" 0 0))
  (Utilities|Array|AddUnique (Variables|Default|GetItemsRef) _returnvalue))

(fn TakeItem
  (bind (_array_element _array_index) (Utilities|Array|ForEachLoopwithBreak (Variables|Default|GetItemsRef))
    (:LoopBody
      (Utilities|IsValid _array_element
        (:Is%20Valid
          (LocalVariables|SetIndex _array_index))))
    (:Completed
      (if (== (LocalVariables|GetIndex) 100)
        (return 0)
        (else
          (LocalVariables|SetPickupClass (Utilities|GetClass (Utilities|Array|Get(acopy) (Variables|Default|GetItemsRef) (LocalVariables|GetIndex))))
          (Actor|DestroyActor (Utilities|Array|Get(acopy) (Variables|Default|GetItemsRef) (LocalVariables|GetIndex)))
          (Utilities|Array|RemoveIndex (Variables|Default|GetItemsRef) (LocalVariables|GetIndex))
          (return (LocalVariables|GetPickupClass)))))))