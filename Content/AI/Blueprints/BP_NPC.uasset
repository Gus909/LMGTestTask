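; BP_NPC is an AI-driven NPC that receives a random category when play begins.
; On BeginPlay it picks one of three E_Category values, stores it in Category and writes it to its Blackboard along with a fixed starting E_AIState.
; It holds no other active logic: Tick, overlap and the construction script are empty.
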(event EventBeginPlay
  (Variables|Default|SetCategory (Utilities|Enum|ByteToEnumE_Category (Math|Conversions|ToByte(Integer) (Math|Random|RandomIntegerinRange 0 2))))
  (AI|Components|Blackboard|SetValueasEnum (AI|GetBlackboard 0) (Utilities|Name|MakeLiteralName "Category") (Variables|Default|GetCategory))
  (AI|Components|Blackboard|SetValueasEnum (AI|GetBlackboard 0) (Utilities|Name|MakeLiteralName "State") (Utilities|Enum|LiteralenumE_AIState "NewEnumerator1")))

(event Collision|EventActorBeginOverlap
  (params (OtherActor :type Actor%20Object%20Reference)))

(event EventTick
  (params (DeltaSeconds :type Float%20%28single-precision%29)))

(fn ConstructionScript)